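; BP_Scientist is an AI-controlled scientist driven by the BT_Scientist behavior tree.
; On BeginPlay it starts the tree and copies its FWanderingRange variable into the Blackboard.
; Its PawnSensing component feeds the Blackboard, writing the location of any seen BP_Beta as the player location and the location of any heard noise as the hearing location.
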(event `self.ReceiveBeginPlay`
  (`AIController.RunBehaviorTree` (`AIBlueprintHelperLibrary.GetAIController` self) "/Game/Blueprints/IA/BT_Scientist.BT_Scientist")
  (`BlackboardComponent.SetValueAsFloat` (`AIBlueprintHelperLibrary.GetBlackboard` null) "f_WanderingRange" (`self.f_WanderingRange`)))

(event `self.PawnSensing.OnSeePawn`
  (params (Pawn :type "Pawn Object Reference"))
  (bind _asbp_beta (cast `/Game/Blueprints/Character/BP_Beta` Pawn))
  (`BlackboardComponent.SetValueAsVector` (`AIBlueprintHelperLibrary.GetBlackboard` null) "v3_PlayerLocation" (`self.K2_GetActorLocation` _asbp_beta)))

(event `self.PawnSensing.OnHearNoise`
  (params (Instigator :type "Pawn Object Reference") (Location :type "Vector Structure (by ref)") (Volume :type "Float (single-precision)"))
  (`BlackboardComponent.SetValueAsVector` (`AIBlueprintHelperLibrary.GetBlackboard` null) "v3_HearingLocation" Location))

(fn `UserConstructionScript`)