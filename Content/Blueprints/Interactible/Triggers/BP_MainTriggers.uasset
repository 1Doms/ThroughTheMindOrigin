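; BP_MainTriggers is an interactible trigger, apparently a base for other triggers, that relays activation to other actors.
; On Interaction, it sends ActivatedMessage to its parent actor when one is valid, as when placed through a Child Actor Component.
; Otherwise, it sends the message to every entry in its ActorLink array, if that array is not empty.
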(event `self.ReceiveTick`
  (params (DeltaSeconds :type "Float (single-precision)"))
  (`parent.ReceiveTick` DeltaSeconds))

(event `/Game/Blueprints/Interactible/BPI_Interaction.Interaction`
  (bind _returnvalue (`self.GetParentActor`))
  (bind _actorlink (`self.ActorLink`))
  (`/Engine/EditorBlueprintResources/StandardMacros.IsValid` _returnvalue
    (:`Is Valid`
      (message `/Game/Blueprints/Interactible/BPI_Interaction.Activated` _returnvalue))
    (:`Is Not Valid`
      (if (`KismetArrayLibrary.Array_IsValidIndex` _actorlink)
        (for _array_element _actorlink
          (message `/Game/Blueprints/Interactible/BPI_Interaction.Activated` _array_element))))))

(fn `UserConstructionScript`
  (`parent.UserConstructionScript`))