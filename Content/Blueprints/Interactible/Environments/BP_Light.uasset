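; BP_Light is an interactible environment light that shows or hides its SpotLight when activated.
; It extends a parent's activation events, branching on SEnviroInteract.TriggerType, with its initial state read from the SpotLight's visibility.
; Interactible mode toggles the light on each activation.
; Overlap mode turns it on at activation and, after deactivation, uses a retriggerable delay to turn it off only if the overlap has not resumed.
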(event `self.ReceiveBeginPlay`
  (`parent.ReceiveBeginPlay`)
  (set `self.b_isActive?` (`SceneComponent.bVisible` (`self.SpotLight`))))

(event `self.Child_Activated`
  (switch `/Game/Blueprints/Interactible/Triggers/E_TriggerType` (`.TriggerType_19_E614F3654BF7F795CBF240A4735357AB` (break `/Game/Blueprints/Interactible/Environments/S_EnvironmentInteractible` (`self.S_ EnviroInteract`)))
    (:`NewEnumerator0`
      (if (`self.b_isActive?`)
        (set `self.b_isActive?` false)
        (`self.TurnOffLight`)
        (else
          (set `self.b_isActive?` true :!label _label)
          (`self.TurnOnLight`))))
    (:`NewEnumerator1`
      (set `self.b_isOverlap` true)
      (goto _label))))

(event `self.Child_Desactivated`
  (switch `/Game/Blueprints/Interactible/Triggers/E_TriggerType` (`.TriggerType_19_E614F3654BF7F795CBF240A4735357AB` (break `/Game/Blueprints/Interactible/Environments/S_EnvironmentInteractible` (`self.S_ EnviroInteract`)))
    (:`NewEnumerator1`
      (set `self.b_isOverlap` false)
      (`KismetSystemLibrary.RetriggerableDelay` 1.5)
      (if (not (`self.b_isOverlap`))
        (`self.TurnOffLight`)))))

(fn `TurnOffLight`
  (`SceneComponent.SetVisibility` (`self.SpotLight`) false false))

(fn `TurnOnLight`
  (`SceneComponent.SetVisibility` (`self.SpotLight`) true false))

(fn `UserConstructionScript`
  (`parent.UserConstructionScript`))