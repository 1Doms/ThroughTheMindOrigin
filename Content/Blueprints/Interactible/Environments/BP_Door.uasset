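; Environment door that slides its static mesh up when activated and back down to close, via an eased MoveComponentTo.
; Responds to ChildActivated and ChildDesactivated according to the trigger type in SEnviroInteract.
; Interactible triggers toggle the door; Overlap triggers open it, then close it after a retriggerable delay if the overlap has not resumed.
; The OpenDoor and CloseDoor functions are empty stubs.
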(event `self.ReceiveBeginPlay`
  (`parent.ReceiveBeginPlay`)
  (set `self.v3_CurrentLocation` (0.0 0.0 0.0)))

(event `self.Child_Activated`
  (switch `/Game/Blueprints/Interactible/Triggers/E_TriggerType` (`.TriggerType_19_E614F3654BF7F795CBF240A4735357AB` (break `/Game/Blueprints/Interactible/Environments/S_EnvironmentInteractible` (`self.S_ EnviroInteract`)))
    (:`NewEnumerator0`
      (if (`self.b_isActive?`)
        (set `self.b_isActive?` false)
        (else
          (set `self.b_isActive?` true :!label _label))))
    (:`NewEnumerator1`
      (set `self.b_isOverlap` true)
      (goto _label)))
  (`KismetSystemLibrary.MoveComponentTo` (`self.StaticMesh`) (select `bool` (`self.b_isActive?`) :`true` (0.0 0.0 256.0) :!type "Vector Structure") (struct) true true 3.0 :!label _label_2))

(event `self.Child_Desactivated`
  (switch `/Game/Blueprints/Interactible/Triggers/E_TriggerType` (`.TriggerType_19_E614F3654BF7F795CBF240A4735357AB` (break `/Game/Blueprints/Interactible/Environments/S_EnvironmentInteractible` (`self.S_ EnviroInteract`)))
    (:`NewEnumerator1`
      (set `self.b_isOverlap` false)
      (`KismetSystemLibrary.RetriggerableDelay` 1.5)
      (if (not (`self.b_isOverlap`))
        (set `self.b_isActive?` false)
        (goto _label_2)))))

(fn `Close Door`)

(fn `Open Door`)

(fn `UserConstructionScript`
  (`parent.UserConstructionScript`))