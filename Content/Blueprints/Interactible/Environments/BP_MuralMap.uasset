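; Interactible mural map environment actor that pulls the player into position facing it when interacted with.
; Interaction plays a timeline that lerps the player character toward the StaticMesh component's X and Y, keeping the player's height, with sweep enabled.
; Character rotation snaps to look at the actor on each update, since the rotator lerp from camera rotation uses a fixed alpha of 1.
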(event `/Game/Blueprints/Interactible/BPI_Interaction.Interaction`
  (bind _returnvalue (`GameplayStatics.GetPlayerCharacter` 0))
  (bind _returnvalue_2 (`self.K2_GetActorLocation` _returnvalue))
  (bind (_returnvalue_x _returnvalue_y) (`KismetMathLibrary.BreakVector` (`SceneComponent.K2_GetComponentLocation` (`self.StaticMesh`))))
  (bind (_direction _newtrack_0) (`Timeline|Lerp` :!via `PlayFromStart`)
    (:`Update`
      (`self.K2_SetActorLocationAndRotation` _returnvalue (`KismetMathLibrary.VLerp` _returnvalue_2 (`KismetMathLibrary.MakeVector` _returnvalue_x _returnvalue_y (.z _returnvalue_2)) _newtrack_0) (`KismetMathLibrary.RLerp` (`PlayerCameraManager.GetCameraRotation` (`GameplayStatics.GetPlayerCameraManager` 0)) (`KismetMathLibrary.FindLookAtRotation` _returnvalue_2 (`self.K2_GetActorLocation`)) 1.0) true false))))

(fn `UserConstructionScript`
  (`parent.UserConstructionScript`))