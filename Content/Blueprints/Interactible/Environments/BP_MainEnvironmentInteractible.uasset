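; Base actor for environment interactibles, meant to be subclassed with specific activation behaviour.
; The construction script looks up a trigger data table row, sets the trigger child actor's class from it and copies the trigger type into the interactible's settings struct.
; Activated and Desactived events forward to empty ChildActivated and ChildDesactivated functions that serve as hooks for child Blueprints.
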(event `self.ReceiveTick`
  (params (DeltaSeconds :type "Float (single-precision)"))
  (`parent.ReceiveTick` DeltaSeconds))

(event `/Game/Blueprints/Interactible/BPI_Interaction.Activated`
  (`self.Child_Activated`))

(event `/Game/Blueprints/Interactible/BPI_Interaction.Desactived`
  (`self.Child_Desactivated`))

(fn `Child_Activated`)

(fn `Child_Desactivated`)

(fn `UserConstructionScript`
  (bind (_description _staticmesh _condition _sfxs _vfxs) (break `/Game/Blueprints/Interactible/Environments/S_EnvironmentInteractible` (`self.S_ EnviroInteract`)))
  (bind (_datatable _rowname) (break `DataTableRowHandle` (`self.DT_Trigger`)))
  (bind _returnvalue (`|GetDataTableRow` _datatable _rowname)
    (:`then`
      (bind (_description_2 _blueprint _triggertype) (break `/Game/Blueprints/Interactible/Triggers/S_Triggers` _returnvalue))
      (`ChildActorComponent.SetChildActorClass` (`self.BP_MainTriggers`) _blueprint)
      (set `self.S_ EnviroInteract` (make `/Game/Blueprints/Interactible/Environments/S_EnvironmentInteractible` _description _staticmesh _condition _sfxs _vfxs _triggertype)))))